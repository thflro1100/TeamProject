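; Prop pawn for a Propnight-style mode that a survivor possesses to disguise as an object, with right-click returning control to the survivor character.
; Movement uses spring-arm-relative forces and a jump impulse on the physics-simulated mesh.
; Left-click traces from the camera and copies the mesh and material of actors tagged "prop".
; Req/Res event pairs relay transforms and possession changes, which toggle mesh visibility, physics and collision.
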(event `req_test`
  (bind _my_survivor_character (`self.My Survivor Character`))
  ;[0.1823 0.1823 0.1823] 코멘트
  (`/Engine/EditorBlueprintResources/StandardMacros.IsValid` _my_survivor_character
    (:`Is Valid`
      (`KismetSystemLibrary.PrintString` (`KismetStringLibrary.Concat_StrStr` (`KismetSystemLibrary.GetDisplayName` _my_survivor_character) " / " (`KismetSystemLibrary.GetObjectName` _my_survivor_character)) true true (struct :`G` 0.66 :`B` 1.0 :`A` 1.0) 5.0))
    (:`Is Not Valid`
      (`KismetSystemLibrary.PrintString` "None" true true (struct :`R` 1.0 :`A` 1.0) 5.0))))

(event `Key|E`
  (params (Key :type "Key Structure"))
  (bind (_returnvalue_roll _returnvalue_pitch _returnvalue_yaw) (`KismetMathLibrary.BreakRotator` (`SceneComponent.K2_GetComponentRotation` (`self.SpringArm`))))
  ;[0.1823 0.1823 0.1823] 코멘트
  (:`Pressed`
    (`SceneComponent.K2_SetWorldRotation` :`self` (`self.Static Mesh`))
    (`Controller.SetControlRotation` (`self.GetController`) (`KismetMathLibrary.MakeRotator` _returnvalue_roll _returnvalue_pitch _returnvalue_yaw))
    (`KismetSystemLibrary.PrintString` (`KismetStringLibrary.Conv_DoubleToString` _returnvalue_yaw))))

(event `Key|Two`
  (params (Key :type "Key Structure"))
  ;[0.1823 0.1823 0.1823] 코멘트
  (:`Pressed`
    (`self.req_test`)))

(event `/Game/Level/Game/GameMode/SurvivorCharacter/Propnight/Blueprints/Interface/IF_Set_Character.Set_Character`
  (params (SurvivorCharacter :type "Character Object Reference"))
  ;[1 1 1] 코멘트
  (bind _asbp_survivor_character_final (cast `/Game/Level/Game/GameMode/SurvivorCharacter/Propnight/GameMode/PlayLevel/BP_SurvivorCharacterFinal` SurvivorCharacter)
    (:`then`
      (set `self.My Survivor Character` _asbp_survivor_character_final))
    (:`CastFailed`
      (`KismetSystemLibrary.PrintString` "SurvivorCharacter Cast Failed" true true (struct :`R` 1.0 :`B` 0.062734 :`A` 1.0)))))

(event `req_CharacterCast`
  (params (NewParam :type "Character Object Reference"))
  ;[1 1 1 1 70] 스폰이벤트
)

(event `res_CharacterCast`
  (params (NewParam :type "/Game/Level/Game/GameMode/SurvivorCharacter/Propnight/GameMode/PlayLevel/BP_SurvivorCharacterFinal Object Reference"))
  ;[1 1 1 1 70] 스폰이벤트
)

(event `self.ReceiveBeginPlay`
  ;[1 1 1 1 70] 스폰이벤트
  ;;[1 1 1] 코멘트
)

(event `req_Server Loc Rot`
  (params (`Static Mesh` :type "StaticMeshComponent Object Reference") (`Mesh Location` :type "Vector Structure") (`Mesh Rotation` :type "Rotator Structure") (`Spring Arm` :type "SpringArmComponent Object Reference") (`Spring Arm Rotation` :type "Rotator Structure"))
  ;[1 1 1 1 70] Tick) 서버에 캐릭터의 위치값 회전값 전달
  ;;[1 0 0] (서버->클라)
  (`self.res_Server Loc Rot` `Static Mesh` `Mesh Location` `Mesh Rotation` `Spring Arm` `Spring Arm Rotation`))

(event `res_Server Loc Rot`
  (params (`Static Mesh` :type "StaticMeshComponent Object Reference") (`Mesh Location` :type "Vector Structure") (`Mesh Rotation` :type "Rotator Structure") (`Spring Arm` :type "SpringArmComponent Object Reference") (`Spring Arm Rotation` :type "Rotator Structure"))
  ;[1 1 1 1 70] Tick) 서버에 캐릭터의 위치값 회전값 전달
  ;;[1 1 1] 전달받은 위치값을 각 클라이언트에 업데이트
  (`SceneComponent.K2_SetWorldLocationAndRotation` `Static Mesh` `Mesh Location` `Mesh Rotation` false false)
  (`SceneComponent.K2_SetWorldRotation` `Spring Arm` `Spring Arm Rotation` false false))

(event `self.ReceiveTick`
  (params (DeltaSeconds :type "Float (single-precision)"))
  ;[1 1 1 1 70] Tick) 서버에 캐릭터의 위치값 회전값 전달
  ;;[1 1 1] SpringArm의 회전값을
  ;; 컨트롤러의 Y,Z 값으로 설정되며 X는 0으로 고정
)

(event `Key|LeftMouseButton`
  (params (Key :type "Key Structure"))
  ;[1 1 1] 코멘트
  ;;[1 1 1 1 70] 다른 프롭으로 변신 (좌클릭)
  ;;;[1 1 1] 다른 프롭으로 변신(클라->서버)
  (:`Pressed`
    (`self.req_transform`)))

(event `res_transform`
  (params (`Static Mesh` :type "StaticMesh Object Reference") (`Material Interface` :type "MaterialInterface Object Reference"))
  ;[1 1 1] 코멘트
  ;;[1 1 1 1 70] 다른 프롭으로 변신 (좌클릭)
  ;;;[1 1 1] 서버에서 전달받은 스테틱매시, 머터리얼로 변경
  (`self.Set Static Mesh` `Static Mesh` `Material Interface`))

(event `req_transform`
  (bind _camera (`self.Camera`))
  (bind _returnvalue (`SceneComponent.K2_GetComponentLocation` _camera))
  (bind _returnvalue_2 (`SceneComponent.GetForwardVector` _camera))
  ;[1 1 1] 코멘트
  ;;[1 1 1 1 70] 다른 프롭으로 변신 (좌클릭)
  ;;;[1 0 0] 클라->서버)
  ;;;;[1 1 1] 카메라 보는 방향으로 라인트레이스 발사
  (bind _outhit (`KismetSystemLibrary.LineTraceSingle` :`Start` (+ _returnvalue (* _returnvalue_2 700)) :`End` (+ _returnvalue (* _returnvalue_2 1200)) :`TraceChannel` "TraceTypeQuery1" :`DrawDebugType` "ForDuration"))
  ;;;;[1 1 1] 대상이 Prop 태그를 가지고 있다면
  (`/Engine/EditorBlueprintResources/StandardMacros.IsValid` (`.HitActor` (`GameplayStatics.BreakHitResult` _outhit))
    (:`Is Valid`
      (if (`self.ActorHasTag` (`.HitActor` (`GameplayStatics.BreakHitResult` _outhit)) "prop")
        (bind _staticmesh (`StaticMeshComponent.StaticMesh` (`self.GetComponentByClass` (`.HitActor` (`GameplayStatics.BreakHitResult` _outhit)) "/Script/Engine.StaticMeshComponent")))
        ;;;;[1 1 1] 스테틱매시 컴포넌트를 추출해서 클라이언트에 전달
        (`self.res_transform` _staticmesh (`StaticMesh.GetMaterial` _staticmesh 0))))))

(event `InputAction|Jump`
  (params (Key :type "Key Structure"))
  ;[1 1 1 1 70] 점프
  (:`Pressed`
    (if (`self.IsGround`)
      (set `self.IsGround` false)
      (`PrimitiveComponent.AddImpulseAtLocation` (`self.Static Mesh`) (0.0 0.0 40000.0) (`SceneComponent.K2_GetComponentLocation` (`self.Static Mesh`)) "None")))
  (:`Released`
    (set `self.IsGround` false)))

(event `InputAxis|MoveForward` :overrideparent false
  (params (AxisValue :type "Float (single-precision)"))
  ;[1 1 1 1 70] 이동 (WASD)
  (`self.ServerMoveFoward` AxisValue))

(event `self.Static Mesh.OnComponentHit`
  (params (HitComponent :type "PrimitiveComponent Object Reference") (OtherActor :type "Actor Object Reference") (OtherComp :type "PrimitiveComponent Object Reference") (NormalImpulse :type "Vector Structure") (Hit :type "HitResult Structure (by ref)"))
  ;[1 1 1 1 70] 점프
  (`/Engine/EditorBlueprintResources/StandardMacros.IsValid` OtherActor
    (:`Is Valid`
      (set `self.IsGround` true))
    (:`Is Not Valid`
      (set `self.IsGround` false))))

(event `커스텀이벤트_0`
  ;[1 1 1 1 70] 프랍_ 굴리기(폐기)
)

(event `InputAxis|MoveRight` :overrideparent false
  (params (AxisValue :type "Float (single-precision)"))
  ;[1 1 1 1 70] 이동 (WASD)
  (`self.ServerMoveRight` AxisValue))

(event `ServerMoveFoward`
  (params (InputPin :type "Float (double-precision)"))
  (`self.MoveFoward` InputPin))

(event `req_Client Possess`
  ;[1 1 1] 코멘트
  ;;[1 1 1 1 70] 빙의 될때 이벤트
  ;;;[1 0 0] (서버->클라)
  (`self.res_Client Possess`))

(event `self.ReceivePossessed`
  (params (NewController :type "Controller Object Reference"))
  ;[1 1 1] 코멘트
  ;;[1 1 1 1 70] 빙의 될때 이벤트
  (`self.req_Client Possess`))

(event `res_Client Possess`
  (bind _static_mesh (`self.Static Mesh`))
  ;[1 1 1] 코멘트
  ;;[1 1 1 1 70] 빙의 될때 이벤트
  ;;;[1 1 1] 보이기
  (`SceneComponent.SetVisibility` _static_mesh true false)
  (`PrimitiveComponent.SetCollisionEnabled` _static_mesh "QueryAndPhysics")
  (`PrimitiveComponent.SetSimulatePhysics` _static_mesh true)
  (`PrimitiveComponent.SetCollisionResponseToChannel` (`self.Static Mesh`) "ECC_Pawn" "ECR_Block"))

(event `ServerMoveRight`
  (params (InputPin :type "Float (double-precision)"))
  (`self.MoveRight` InputPin))

(event `res_to human_Server`
  (params (controller :type "Controller Object Reference") (`Survivor Character` :type "Character Object Reference") (NewParam :type "Rotator Structure"))
  (bind (_returnvalue_x _returnvalue_y _returnvalue_z) (`KismetMathLibrary.BreakVector` (`self.K2_GetActorLocation` self)))
  ;[1 1 1] 코멘트
  ;;[1 1 1 1 70] 현재 캐릭터의 빙의를 풀고 원래 캐릭터로 빙의 (우클릭)
  ;;;[1 0 0] 서버에서 이벤트 실행
  (`self.K2_SetActorLocation` (`self.My Survivor Character`) (`KismetMathLibrary.MakeVector` _returnvalue_x _returnvalue_y (+ _returnvalue_z 100.0)) false false)
  ;;;;[0 1 1] 빙의해제 -> 다른캐릭터에 빙의
  (`Controller.Possess` (`self.GetController`) (`self.My Survivor Character`)))

(event `Key|RightMouseButton`
  (params (Key :type "Key Structure"))
  ;[1 1 1] 코멘트
  ;;[1 1 1 1 70] 현재 캐릭터의 빙의를 풀고 원래 캐릭터로 빙의 (우클릭)
  ;;;[1 1 1] 변신 해제
  (:`Pressed`
    (`SceneComponent.K2_SetWorldRotation` :`self` (`self.Static Mesh`))
    (`Controller.SetControlRotation` (`self.GetController`) (`SceneComponent.K2_GetComponentRotation` (`self.SpringArm`)))
    (`self.res_to human_Server` null)))

(event `req_Client UnPossess`
  ;[1 1 1] 코멘트
  ;;[1 1 1 1 70] 빙의 풀렸을때 이벤트
  ;;;[1 0 0] (서버->클라)
  (`self.res_Client UnPossess`))

(event `res_Client UnPossess`
  (bind _static_mesh (`self.Static Mesh`))
  ;[1 1 1] 코멘트
  ;;[1 1 1 1 70] 빙의 풀렸을때 이벤트
  ;;;[1 1 1] 숨기기
  (`SceneComponent.SetVisibility` _static_mesh false false)
  (`PrimitiveComponent.SetSimulatePhysics` _static_mesh false)
  (`PrimitiveComponent.SetCollisionEnabled` _static_mesh "NoCollision")
  (`PrimitiveComponent.SetCollisionResponseToChannel` (`self.Static Mesh`) "ECC_Pawn" "ECR_Ignore"))

(event `self.ReceiveUnpossessed`
  (params (OldController :type "Controller Object Reference"))
  ;[1 1 1] 코멘트
  ;;[1 1 1 1 70] 빙의 풀렸을때 이벤트
  (`self.req_Client UnPossess`))

(event `Key|Q`
  (params (Key :type "Key Structure"))
  (bind (_relativerotation_roll _relativerotation_pitch _relativerotation_yaw) (`KismetMathLibrary.BreakRotator` (`SceneComponent.RelativeRotation` (`self.SpringArm`))))
  ;[1 1 1 1 70] 위치 정렬 (Q키)
  (:`Pressed`
    (`SceneComponent.K2_SetRelativeRotation` (`self.Static Mesh`) (`KismetMathLibrary.MakeRotator` 0.0 0.0 _relativerotation_yaw) false false)))

(fn `MoveFoward`
  (params (InputPin :type "Float (double-precision)"))
  (bind (_relativerotation_roll _relativerotation_pitch _relativerotation_yaw) (`KismetMathLibrary.BreakRotator` (`SceneComponent.RelativeRotation` (`self.SpringArm`))))
  (if (`SceneComponent.IsSimulatingPhysics` (`self.Static Mesh`) "None")
    (`PrimitiveComponent.AddForce` (`self.Static Mesh`) (* (`KismetMathLibrary.GetForwardVector` (`KismetMathLibrary.MakeRotator` _relativerotation_roll 0.0 _relativerotation_yaw)) (* InputPin 1500.0)) "None" true)))

(fn `MoveRight`
  (params (InputPin :type "Float (double-precision)"))
  (bind (_relativerotation_roll _relativerotation_pitch _relativerotation_yaw) (`KismetMathLibrary.BreakRotator` (`SceneComponent.RelativeRotation` (`self.SpringArm`))))
  (if (`SceneComponent.IsSimulatingPhysics` (`self.Static Mesh`) "None")
    (`PrimitiveComponent.AddForce` (`self.Static Mesh`) (* (`KismetMathLibrary.GetRightVector` (`KismetMathLibrary.MakeRotator` _relativerotation_roll 0.0 _relativerotation_yaw)) (* InputPin 1500.0)) "None" true)))

(fn `OnRep_Pitch`)

(fn `Set Static Mesh`
  (params (GetStaticMesh :type "StaticMesh Object Reference") (GetMaterial :type "MaterialInterface Object Reference") (SurvivorCharacter :type "Character Object Reference"))
  ;[1 1 1] SurvivorCharacter 혹은
  ; PropCharacter 에서
  ; 상호작용키(F) 누를때 함수 실행
  ;[1 1 1] 스테틱매시를 가져온다.
  (`StaticMeshComponent.SetStaticMesh` (`self.Static Mesh`) GetStaticMesh)
  (`PrimitiveComponent.SetMaterial` (`self.Static Mesh`) 0 GetMaterial)
  ;[1 1 1] 매쉬의 콜리젼 상태 확인 후
  ; (콜리전상태 == 빙의상태)
  (if (not (`PrimitiveComponent.K2_IsCollisionEnabled` (`self.Static Mesh`)))
    ;[1 1 1] 콜리젼이 꺼져있으면 SpringArm의 회전값을
    ; SurvivorCharacter의 회전값으로 설정한다.
    (`SceneComponent.K2_SetRelativeRotation` (`self.SpringArm`) (`self.GetControlRotation` SurvivorCharacter) false false)))

(fn `UserConstructionScript`)